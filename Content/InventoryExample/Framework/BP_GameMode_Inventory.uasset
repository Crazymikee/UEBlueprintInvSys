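; Example game mode that persists player and world-container inventories through BP_SaveGame_InventoryExample save slots.
; On restart it initializes the PlayerState's AC_InventoryHandler from the save, and on logout writes it back.
; BeginPlay and EndPlay load and save World Container handlers found via InventoryInterfaceCore.
; Missing saves are seeded with default inventory; all players share one fixed slot, all containers another.
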(event EventOnLogout
  (params (ExitingController :type Controller%20Object%20Reference))
  (bind _playerstate (Variables|/Script/Engine.Controller|GetPlayerState ExitingController))
  (bind _returnvalue (Actor|GetComponentbyClass _playerstate "/Game/InventoryCore/Components/AC_InventoryHandler.AC_InventoryHandler_C"))
  (|CallParentFunction ExitingController)
  (bind _returnvalue_2 (SaveGame|LoadGamefromSlot "InventoryExample"))
  (Utilities|IsValid _returnvalue_2
    (:Is%20Valid
      (bind _asbp_save_game_inventory_example (Utilities|Casting|CastToBP_SaveGame_InventoryExample _returnvalue_2))
      (Variables|/Game/InventoryExample/Blueprints/BP_SaveGame_InventoryExample.BP_SaveGame_InventoryExample_C|SetSaved%20Inventory _asbp_save_game_inventory_example (Utilities|Struct|MakeSavedInventory (Variables|/Game/InventoryCore/Components/AC_InventoryHandler.AC_InventoryHandler_C|GetMain%20Inventory _returnvalue) (Variables|/Game/InventoryCore/Components/AC_InventoryHandler.AC_InventoryHandler_C|GetEquipped%20Inventory _returnvalue)))
      (SaveGame|SaveGametoSlot _asbp_save_game_inventory_example "InventoryExample"))))

(event EventPostLogin
  (params (NewPlayer :type Player%20Controller%20Object%20Reference))
  (Utilities|IsValid (Actor|GetComponentbyClass NewPlayer "/Game/InventoryCore/Components/AC_InventoryHandler.AC_InventoryHandler_C")))

(event EventEndPlay
  (params (EndPlayReason :type EEndPlayReason%20Enum :default "Destroyed"))
  (CallFunction|HandleContainerPersistence))

(event EventOnRestartPlayer
  (params (NewPlayer :type Controller%20Object%20Reference))
  (bind _playerstate (Variables|/Script/Engine.Controller|GetPlayerState NewPlayer))
  (bind _returnvalue (Actor|GetComponentbyClass _playerstate "/Game/InventoryCore/Components/AC_InventoryHandler.AC_InventoryHandler_C"))
  (|CallParentFunction NewPlayer)
  (Utilities|IsValid _returnvalue
    (:Is%20Valid
      (bind _returnvalue_2 (SaveGame|LoadGamefromSlot "InventoryExample" :!label _label))
      (Utilities|IsValid _returnvalue_2
        (:Is%20Valid
          (bind _asbp_save_game_inventory_example (Utilities|Casting|CastToBP_SaveGame_InventoryExample _returnvalue_2))
          (Default|ServerFuncInitializeInventory _returnvalue (Variables|/Game/InventoryExample/Blueprints/BP_SaveGame_InventoryExample.BP_SaveGame_InventoryExample_C|GetSaved%20Inventory _asbp_save_game_inventory_example)))
        (:Is%20Not%20Valid
          ;[1 0 0.8323] Create Example Saved Inventory Data & Reload
          (bind _returnvalue_3 (SaveGame|CreateSaveGameObject "/Game/InventoryExample/Blueprints/BP_SaveGame_InventoryExample.BP_SaveGame_InventoryExample_C"))
          (Variables|/Game/InventoryExample/Blueprints/BP_SaveGame_InventoryExample.BP_SaveGame_InventoryExample_C|SetSaved%20Inventory _returnvalue_3 (Default|GetDefaultInventory _returnvalue))
          (bind _returnvalue_4 (SaveGame|SaveGametoSlot _returnvalue_3 "InventoryExample"))
          (if _returnvalue_4
            (goto _label)))))))

(event EventBeginPlay
  (bind _outactors (Actor|GetAllActorswithInterface "/Game/InventoryCore/Interface/InventoryInterfaceCore.InventoryInterfaceCore_C"))
  (for _array_element _outactors
    (Utilities|IsValid (Actor|GetComponentbyClass _array_element "/Game/InventoryCore/Components/AC_InventoryHandler.AC_InventoryHandler_C")
      (:Is%20Valid
        (switch Utilities|FlowControl|Switch|SwitchonInventoryCompType (Variables|/Game/InventoryCore/Components/AC_InventoryHandler.AC_InventoryHandler_C|GetComponent%20Type (Actor|GetComponentbyClass _array_element "/Game/InventoryCore/Components/AC_InventoryHandler.AC_InventoryHandler_C"))
          (:NewEnumerator1
            (bind _returnvalue (SaveGame|LoadGamefromSlot "ContainerExample" :!label _label))
            (Utilities|IsValid _returnvalue
              (:Is%20Valid
                (bind _asbp_save_game_inventory_example (Utilities|Casting|CastToBP_SaveGame_InventoryExample _returnvalue))
                (Default|ServerFuncInitializeInventory (Actor|GetComponentbyClass _array_element "/Game/InventoryCore/Components/AC_InventoryHandler.AC_InventoryHandler_C") (Variables|/Game/InventoryExample/Blueprints/BP_SaveGame_InventoryExample.BP_SaveGame_InventoryExample_C|GetSaved%20Inventory _asbp_save_game_inventory_example)))
              (:Is%20Not%20Valid
                ;[1 0 0.8323] Create Example Saved Inventory Data & Reload
                (bind _returnvalue_2 (SaveGame|CreateSaveGameObject "/Game/InventoryExample/Blueprints/BP_SaveGame_InventoryExample.BP_SaveGame_InventoryExample_C"))
                (Variables|/Game/InventoryExample/Blueprints/BP_SaveGame_InventoryExample.BP_SaveGame_InventoryExample_C|SetSaved%20Inventory _returnvalue_2 (Default|GetDefaultInventory (Actor|GetComponentbyClass _array_element "/Game/InventoryCore/Components/AC_InventoryHandler.AC_InventoryHandler_C")))
                (bind _returnvalue_3 (SaveGame|SaveGametoSlot _returnvalue_2 "ContainerExample"))
                (if _returnvalue_3
                  (goto _label))))))))))

(fn ConstructionScript)

(fn HandleContainerPersistence
  (bind _outactors (Actor|GetAllActorswithInterface "/Game/InventoryCore/Interface/InventoryInterfaceCore.InventoryInterfaceCore_C"))
  (for _array_element _outactors
    (Utilities|IsValid (Actor|GetComponentbyClass _array_element "/Game/InventoryCore/Components/AC_InventoryHandler.AC_InventoryHandler_C")
      (:Is%20Valid
        (switch Utilities|FlowControl|Switch|SwitchonInventoryCompType (Variables|/Game/InventoryCore/Components/AC_InventoryHandler.AC_InventoryHandler_C|GetComponent%20Type (Actor|GetComponentbyClass _array_element "/Game/InventoryCore/Components/AC_InventoryHandler.AC_InventoryHandler_C"))
          (:NewEnumerator1
            (bind _returnvalue (SaveGame|LoadGamefromSlot "ContainerExample" :!label _label))
            (Utilities|IsValid _returnvalue
              (:Is%20Valid
                (bind _asbp_save_game_inventory_example (Utilities|Casting|CastToBP_SaveGame_InventoryExample _returnvalue))
                (Variables|/Game/InventoryExample/Blueprints/BP_SaveGame_InventoryExample.BP_SaveGame_InventoryExample_C|SetSaved%20Inventory _asbp_save_game_inventory_example (Utilities|Struct|MakeSavedInventory (Variables|/Game/InventoryCore/Components/AC_InventoryHandler.AC_InventoryHandler_C|GetMain%20Inventory (Actor|GetComponentbyClass _array_element "/Game/InventoryCore/Components/AC_InventoryHandler.AC_InventoryHandler_C")) (Variables|/Game/InventoryCore/Components/AC_InventoryHandler.AC_InventoryHandler_C|GetEquipped%20Inventory (Actor|GetComponentbyClass _array_element "/Game/InventoryCore/Components/AC_InventoryHandler.AC_InventoryHandler_C"))))
                (SaveGame|SaveGametoSlot _returnvalue "ContainerExample"))
              (:Is%20Not%20Valid
                ;[1 0 0.8323] Create Example Saved Inventory Data & Reload
                (bind _returnvalue_2 (SaveGame|CreateSaveGameObject "/Game/InventoryExample/Blueprints/BP_SaveGame_InventoryExample.BP_SaveGame_InventoryExample_C"))
                (Variables|/Game/InventoryExample/Blueprints/BP_SaveGame_InventoryExample.BP_SaveGame_InventoryExample_C|SetSaved%20Inventory _returnvalue_2 (Default|GetDefaultInventory (Actor|GetComponentbyClass _array_element "/Game/InventoryCore/Components/AC_InventoryHandler.AC_InventoryHandler_C")))
                (bind _returnvalue_3 (SaveGame|SaveGametoSlot _returnvalue_2 "ContainerExample"))
                (if _returnvalue_3
                  (goto _label))))))))))