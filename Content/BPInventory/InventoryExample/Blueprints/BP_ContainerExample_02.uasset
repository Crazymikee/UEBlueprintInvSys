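; Example interactable container that shows its equipped inventory items as physical meshes on three slot components.
; The server initializes the inventory handler, serves interaction requests and multicasts equipped-slot changes, while remote clients poll on BeginPlay until data exists.
; Clients spawn cosmetic BP_DroppedItem actors with physics, collision, widget and pickup disabled, attached with optional per-item offsets, replacing or destroying them as slots change.
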(event Custom|MulticastEvent_SlotStateChange
  (params (Index :type Integer) (Valid%20Item :type Boolean) (Inventory%20Item%20Replicated :type Inventory%20Item%20Replicated%20Structure))
  ;[0 0.1701 1] Replicate slot state changes to clients
  (Utilities|AuthoritySwitch (Class|KismetSystemLibrary|IsStandalone) (Ability|HasAuthority)
    (:Remote
      (CallFunction|SlotStateChange Index Valid%20Item Inventory%20Item%20Replicated))))

(event EventBeginPlay
  (bind _ac_inventoryhandler (Variables|Default|GetAC_InventoryHandler))
  (bind _equipped_inventory (Variables|/Game/BPInventory/InventoryCore/Components/InventoryHandler.InventoryHandler_C|GetEquipped%20Inventory _ac_inventoryhandler))
  ;[1 0 0.2825] Initialize client side cosmetic item display
  (|CallParentFunction)
  (Utilities|AuthoritySwitch (Class|KismetSystemLibrary|IsStandalone) (Ability|HasAuthority)
    (:Authority
      (Default|ServerFuncInitializeInventory (Variables|Default|GetAC_InventoryHandler)))
    (:Remote
      (if (Utilities|Array|IsValidIndex _equipped_inventory) :!label _label
        (for (_array_element _array_index) _equipped_inventory
          (CallFunction|SlotStateChange _array_index (CallFunction|CheckValidItem _array_element) _array_element))
        (else
          (Utilities|FlowControl|Delay 0.2)
          (goto _label))))))

(fn ConstructionScript)

(fn SlotStateChange
  (params (Index :type Integer) (Valid%20Item :type Boolean) (Inventory%20Item%20Replicated :type Inventory%20Item%20Replicated%20Structure))
  (bind _slot1 (Variables|Default|Getslot1))
  (bind _slot2 (Variables|Default|Getslot2))
  (bind _slot3 (Variables|Default|Getslot3))
  (bind _itemsocketoffsets (Variables|Default|GetItemSocketOffsets))
  (bind _coredatareference (Utilities|Struct|BreakInventoryItemReplicated Inventory%20Item%20Replicated))
  (bind _returnvalue (Utilities|Select :Index Index :Option%200 _slot1 :Option%201 _slot2 :Option%202 _slot3))
  (bind _returnvalue_2 (Components|GetChildComponent _returnvalue 0))
  (bind (_value _returnvalue_3) (Utilities|Map|Find _itemsocketoffsets (Utilities|Struct|MakeDictionaryDataTableInfo (.rowname _coredatareference) (.datatable _coredatareference))))
  (bind _returnvalue_4 (Components|GetOwner _returnvalue_2))
  (if Valid%20Item
    (Utilities|IsValid _returnvalue_2
      (:Is%20Valid
        (if (not (CallFunction|CheckSameRepItemID (Variables|/Game/BPInventory/InventoryExample/Blueprints/BP_DroppedItem.BP_DroppedItem_C|GetInventory%20Item%20Replicated (.AsBP%20Dropped%20Item (Utilities|Casting|CastToBP_DroppedItem _returnvalue_4))) Inventory%20Item%20Replicated))
          (Actor|DestroyActor _returnvalue_4)
          (bind _returnvalue_5 (Game|SpawnActorfromClass :Class "/Game/BPInventory/InventoryExample/Blueprints/BP_DroppedItem.BP_DroppedItem_C" :SpawnTransform (Transformation|GetWorldTransform _returnvalue) :CollisionHandlingOverride "AlwaysSpawn" :TransformScaleMethod "OverrideRootScale" :Owner self :Inventory%20Item%20Replicated Inventory%20Item%20Replicated :Instigator 0 :!label _label))
          (Default|InventoryItemRepResponse _returnvalue_5 (Variables|/Game/BPInventory/InventoryExample/Blueprints/BP_DroppedItem.BP_DroppedItem_C|GetInventory%20Item%20Replicated _returnvalue_5))
          (Physics|SetSimulatePhysics (Actor|GetComponentsByClass _returnvalue_5 "/Script/Engine.PrimitiveComponent") false)
          (Class|PrimitiveComponent|SetAllUseCCD (Actor|GetComponentsByClass _returnvalue_5 "/Script/Engine.PrimitiveComponent") false)
          (Rendering|SetVisibility (Variables|/Game/BPInventory/InventoryExample/Blueprints/BP_DroppedItem.BP_DroppedItem_C|GetWidget _returnvalue_5) false false)
          (Collision|SetActorEnableCollision _returnvalue_5 false)
          (Variables|/Game/BPInventory/InventoryExample/Blueprints/BP_DroppedItem.BP_DroppedItem_C|SetPickupAttempted _returnvalue_5 true)
          (Transformation|AttachComponentToComponent _returnvalue_5 _returnvalue "None" "SnapToTarget" "SnapToTarget" "SnapToTarget" true)
          (if _returnvalue_3
            (Class|SceneComponent|AddLocalTransform (Actor|GetComponentsByClass _returnvalue_5 "/Script/Engine.PrimitiveComponent") _value false false))))
      (:Is%20Not%20Valid
        (goto _label)))
    (else
      (Utilities|IsValid _returnvalue_2
        (:Is%20Valid
          (Actor|DestroyActor _returnvalue_4))))))

(fn ClientFuncGetSlotInfoWidget
  (params (Slot%20Info :type Slot%20Information%20Structure))
  (return 0))

(fn ClientFuncReceivedHandlerResponse
  (params (Owned%20Handler :type Inventory%20Handler%20Object%20Reference) (Other%20Handler :type Inventory%20Handler%20Object%20Reference))
  (return false))

(fn ClientFuncReceiveInventoryData
  (params (Main%20Inventory :type Array%20of%20Inventory%20Item%20Replicated%20Structures) (Equipped%20Inventory :type Array%20of%20Inventory%20Item%20Replicated%20Structures))
  (return false))

(fn ClientFuncReceiveItemData
  (params (Array%20Type :type InventoryArrayType%20Enum :default "NewEnumerator0") (Index :type Integer) (Inventory%20Item%20Replicated :type Inventory%20Item%20Replicated%20Structure))
  (return false))

(fn ClientFuncSendInitialDatatoInventoryWidget
  (params (Inventory%20Handler :type Inventory%20Handler%20Object%20Reference) (Equipped%20Type%20Array :type Array%20of%20Byte%20Array%20Structures))
  (return false))

(fn GetInteractAllowed
  (return (CallFunction|IsHandlerStateSafe (Variables|Default|GetAC_InventoryHandler))))

(fn GetInventoryHandler
  (return (Variables|Default|GetAC_InventoryHandler)))

(fn GetInventoryItemReplicatedData
  (return ""))

(fn ServerFuncInteractRequest
  (params (Sender :type Actor%20Object%20Reference))
  (Networking|ForceNetUpdate)
  (bind _inventory_handler (Class|InventoryInterfaceCore|GetInventoryHandler(Message) Sender))
  (bind _success (Default|ServerFuncHandlerInteraction _inventory_handler (Variables|Default|GetAC_InventoryHandler)))
  (return _success))

(fn ServerFuncInventoryInitialized
  (params (Inventory%20Handler :type Inventory%20Handler%20Object%20Reference))
  (return false))

(fn ServerFuncInventoryItemDeleted
  (params (Deleted%20Item%20Data :type Inventory%20Item%20Replicated%20Structure))
  (return false))

(fn ServerFuncInventoryItemObtained
  (params (Obtained%20Item%20Data :type Inventory%20Item%20Replicated%20Structure))
  (return false))

(fn ServerFuncInventoryItemProductionResult
  (params (Production%20Successful :type Boolean) (Production%20Data%20Table%20Row :type Data%20Table%20Row%20Handle%20Structure) (Produced%20Items :type Array%20of%20Inventory%20Item%20Replicated%20Structures))
  (return false))

(fn ServerFuncInventorySlotDropped
  (params (Inventory%20Item%20Replicated :type Inventory%20Item%20Replicated%20Structure))
  (return false))

(fn ServerFuncInventorySlotStateChange
  (params (Inventory%20Handler :type Inventory%20Handler%20Object%20Reference) (Array%20Type :type InventoryArrayType%20Enum :default "NewEnumerator0") (Index :type Integer) (Valid%20Item :type Boolean) (Inventory%20Item%20Replicated :type Inventory%20Item%20Replicated%20Structure))
  (switch Utilities|FlowControl|Switch|SwitchonInventoryArrayType Array%20Type
    (:NewEnumerator1
      (CallFunction|MulticastEventSlotStateChange Index Valid%20Item Inventory%20Item%20Replicated)
      (return true))))

(fn ServerFuncInventorySlotValueChange
  (params (Inventory%20Handler :type Inventory%20Handler%20Object%20Reference) (Array%20Type :type InventoryArrayType%20Enum :default "NewEnumerator0") (Index :type Integer) (Inventory%20Item%20Replicated :type Inventory%20Item%20Replicated%20Structure))
  (return true))

(fn SetInventoryItemReplicatedData
  (params (InventoryItemReplicated :type Inventory%20Item%20Replicated%20Structure))
  (return false))