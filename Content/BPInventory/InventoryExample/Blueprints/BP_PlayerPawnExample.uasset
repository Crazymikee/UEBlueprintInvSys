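; Example player pawn demoing the inventory system, using hardcoded key and mouse events for easy migration, with Tick-driven gates for movement.
; Interact keys line-trace from the camera for InventoryInterfaceCore actors and send requests through a server event.
; The PlayerState's inventory handler supplies widgets for Tab toggling, embedded external inventory or transaction panels, and a test production key.
; Interface overrides are mostly stubs, except interaction, UI responses and dropped-item spawning.
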(event Custom|ClientEvent_SendInventoryWidget
  (params (From%20Handler :type AC%20Inventory%20Handler%20Object%20Reference) (To%20Handler :type AC%20Inventory%20Handler%20Object%20Reference))
  (bind _returnvalue (Game|GetPlayerController 0))
  ;[1 1 1] Implemented Event For Interacting With External Handlers (From in this context is the client-owned inventory & To is the external inventory that has been interacted with)
  (Default|ClientEventRemoveInventoryWidget From%20Handler)
  (bind _inventory_widget (Default|ClientFuncGetInventoryWidget To%20Handler))
  (bind _inventory_widget_2 (Default|ClientFuncGetInventoryWidget From%20Handler))
  (bind _asw_inventory_main_example (Utilities|Casting|CastToW_InventoryMain_Example _inventory_widget_2))
  (Widget|Panel|ClearChildren (Variables|/Game/BPInventory/InventoryExample/UI/W_InventoryMain_Example.W_InventoryMain_Example_C|GetOtherWidgetBorder _asw_inventory_main_example))
  (Widget|Panel|AddChild (Variables|/Game/BPInventory/InventoryExample/UI/W_InventoryMain_Example.W_InventoryMain_Example_C|GetOtherWidgetBorder _asw_inventory_main_example) _inventory_widget)
  (Class|InventoryInterfaceCore|ClientFuncReceiveInventoryData(Message) _inventory_widget (Variables|/Game/BPInventory/InventoryCore/Components/AC_InventoryHandler.AC_InventoryHandler_C|GetMain%20Inventory To%20Handler) (Variables|/Game/BPInventory/InventoryCore/Components/AC_InventoryHandler.AC_InventoryHandler_C|GetEquipped%20Inventory To%20Handler))
  (bind _inventory_widget_3 (Default|ClientFuncGetInventoryWidget From%20Handler))
  (if (not (Widget|IsVisible _inventory_widget_3))
    (UserInterface|Viewport|AddtoViewport _inventory_widget_3 0)
    (Input|SetInputModeGameandUI _returnvalue 0 "DoNotLock" true false)
    (Variables|/Script/Engine.PlayerController|SetbShowMouseCursor _returnvalue true)))

(event Custom|ServerEvent_InteractRequest
  (params (Actor :type Actor%20Object%20Reference))
  ;[1 1 1] Simple Demo Actions w/o Project Inputs For Ease Of Migration
  ;;[1 1 1] Attempt to interact with a forward facing actor that has our InventoryCore Interface implemented
  (Class|InventoryInterfaceCore|ServerFuncInteractRequest(Message) Actor (Variables|GetPlayerState)))

(event Custom|ClientEvent_SendTransactionWidget
  (params (Transaction%20Handler :type AC%20Inventory%20Handler%20Object%20Reference))
  (bind _returnvalue (Game|GetPlayerController 0))
  (bind _inventory_handler (Class|InventoryInterfaceCore|GetInventoryHandler(Message) (Variables|GetPlayerState)))
  (Utilities|IsValid _inventory_handler
    (:Is%20Valid
      (switch Utilities|FlowControl|Switch|SwitchonInventoryCompType (Variables|/Game/BPInventory/InventoryCore/Components/AC_InventoryHandler.AC_InventoryHandler_C|GetComponent%20Type Transaction%20Handler)
        (:NewEnumerator0
          (Default|ClientEventRemoveInventoryWidget _inventory_handler :!label _label))
        (:NewEnumerator1
          (goto _label))
        (:NewEnumerator2
          _))
      (bind _inventory_widget (Default|ClientFuncGetInventoryWidget _inventory_handler))
      (bind _transaction_widget (Default|ClientFuncGetTransactionWidget _inventory_handler Transaction%20Handler))
      (bind _asw_inventory_main_example (Utilities|Casting|CastToW_InventoryMain_Example _inventory_widget))
      (Widget|Panel|ClearChildren (Variables|/Game/BPInventory/InventoryExample/UI/W_InventoryMain_Example.W_InventoryMain_Example_C|GetTransactionWidgetBorder _asw_inventory_main_example))
      (Widget|Panel|AddChild (Variables|/Game/BPInventory/InventoryExample/UI/W_InventoryMain_Example.W_InventoryMain_Example_C|GetTransactionWidgetBorder _asw_inventory_main_example) _transaction_widget)
      (if (not (Widget|IsVisible _inventory_widget))
        (UserInterface|Viewport|AddtoViewport _inventory_widget 0)
        (Input|SetInputModeGameandUI _returnvalue 0 "DoNotLock" true false)
        (Variables|/Script/Engine.PlayerController|SetbShowMouseCursor _returnvalue true)))))

(event EventTick
  (params (DeltaSeconds :type Float%20%28single-precision%29))
  (bind _returnvalue (Utilities|ControlRotator))
  (bind _returnvalue_2 (Math|Vector|GetRightVector _returnvalue))
  (bind _returnvalue_3 (Math|Vector|GetForwardVector _returnvalue))
  ;[1 1 1] Simple Demo Actions w/o Project Inputs For Ease Of Migration
  ;;[1 1 1] Move
  (Utilities|FlowControl|Sequence
    (:then_0
      (Utilities|FlowControl|Gate true
        (:Exit
          (Pawn|Input|AddMovementInput _returnvalue_3 1.0 false))))
    (:then_1
      (Utilities|FlowControl|Gate true
        (:Exit
          (Pawn|Input|AddMovementInput _returnvalue_3 -1.0 false))))
    (:then_2
      (Utilities|FlowControl|Gate true
        (:Exit
          (Pawn|Input|AddMovementInput _returnvalue_2 -1.0 false))))
    (:then_3
      (Utilities|FlowControl|Gate true
        (:Exit
          (Pawn|Input|AddMovementInput _returnvalue_2 1.0 false))))))

(event Input|MouseEvents|MouseX
  (params (AxisValue :type Float%20%28single-precision%29))
  ;[1 1 1] Simple Demo Actions w/o Project Inputs For Ease Of Migration
  ;;[1 1 1] Aim
  (Pawn|Input|AddControllerYawInput AxisValue))

(event Input|MouseEvents|MouseY
  (params (AxisValue :type Float%20%28single-precision%29))
  ;[1 1 1] Simple Demo Actions w/o Project Inputs For Ease Of Migration
  ;;[1 1 1] Aim
  (Pawn|Input|AddControllerPitchInput (* AxisValue -1.0)))

(event Input|KeyboardEvents|S
  (params (Key :type Key%20Structure))
  ;[1 1 1] Simple Demo Actions w/o Project Inputs For Ease Of Migration
  ;;[1 1 1] Move
  (:Pressed
    (Utilities|FlowControl|Gate true) ; enters at Open
  )
  (:Released
    (Utilities|FlowControl|Gate true) ; enters at Close
  ))

(event Input|KeyboardEvents|W
  (params (Key :type Key%20Structure))
  ;[1 1 1] Simple Demo Actions w/o Project Inputs For Ease Of Migration
  ;;[1 1 1] Move
  (:Pressed
    (Utilities|FlowControl|Gate true) ; enters at Open
  )
  (:Released
    (Utilities|FlowControl|Gate true) ; enters at Close
  ))

(event Input|KeyboardEvents|Tab
  (params (Key :type Key%20Structure))
  (bind _returnvalue (Game|GetPlayerController 0))
  ;[1 1 1] Display Inventory Widget
  (:Pressed
    (bind _inventory_handler (Class|InventoryInterfaceCore|GetInventoryHandler(Message) (Variables|GetPlayerState)))
    (Utilities|IsValid _inventory_handler
      (:Is%20Valid
        (bind _inventory_widget (Default|ClientFuncGetInventoryWidget _inventory_handler))
        (if (not (Widget|IsVisible _inventory_widget))
          (UserInterface|Viewport|AddtoViewport _inventory_widget 0)
          (Input|SetInputModeGameandUI _returnvalue 0 "DoNotLock" true false)
          (Variables|/Script/Engine.PlayerController|SetbShowMouseCursor _returnvalue true)
          (else
            (Widget|RemovefromParent _inventory_widget)
            (Input|SetInputModeGameOnly _returnvalue false)
            (Variables|/Script/Engine.PlayerController|SetbShowMouseCursor _returnvalue false)))))))

(event Input|KeyboardEvents|E
  (params (Key :type Key%20Structure))
  (bind _hitactor (CallFunction|TracetoFindInventoryActor))
  ;[1 1 1] Simple Demo Actions w/o Project Inputs For Ease Of Migration
  ;;[1 1 1] Attempt to interact with a forward facing actor that has our InventoryCore Interface implemented
  (:Pressed
    (Utilities|IsValid _hitactor
      (:Is%20Valid
        (bind _interactallowed (Class|InventoryInterfaceCore|GetInteractAllowed(Message) _hitactor))
        (if _interactallowed
          (CallFunction|ServerEventInteractRequest _hitactor))))))

(event Input|KeyboardEvents|A
  (params (Key :type Key%20Structure))
  ;[1 1 1] Simple Demo Actions w/o Project Inputs For Ease Of Migration
  ;;[1 1 1] Move
  (:Pressed
    (Utilities|FlowControl|Gate true) ; enters at Open
  )
  (:Released
    (Utilities|FlowControl|Gate true) ; enters at Close
  ))

(event Input|KeyboardEvents|D
  (params (Key :type Key%20Structure))
  ;[1 1 1] Simple Demo Actions w/o Project Inputs For Ease Of Migration
  ;;[1 1 1] Move
  (:Pressed
    (Utilities|FlowControl|Gate true) ; enters at Open
  )
  (:Released
    (Utilities|FlowControl|Gate true) ; enters at Close
  ))

(event Input|MouseEvents|LeftMouseButton
  (params (Key :type Key%20Structure))
  (bind _hitactor (CallFunction|TracetoFindInventoryActor))
  ;[1 1 1] Simple Demo Actions w/o Project Inputs For Ease Of Migration
  ;;[1 1 1] Attempt to interact with a forward facing actor that has our InventoryCore Interface implemented
  (:Pressed
    (Utilities|IsValid _hitactor
      (:Is%20Valid
        (bind _interactallowed (Class|InventoryInterfaceCore|GetInteractAllowed(Message) _hitactor))
        (if _interactallowed
          (CallFunction|ServerEventInteractRequest _hitactor))))))

(event Input|KeyboardEvents|Z
  (params (Key :type Key%20Structure))
  (:Pressed
    (bind _inventory_handler (Class|InventoryInterfaceCore|GetInventoryHandler(Message) (Variables|GetPlayerState)))
    (Default|ServerEventProduceItem _inventory_handler (Utilities|Struct|MakeDataTableRowHandle "/Game/BPInventory/InventoryExample/DT/DT_Production_Examples.DT_Production_Examples" "Production_Bread") (Utilities|Array|MakeArray 0 1))))

(event Input|KeyboardEvents|F
  (params (Key :type Key%20Structure))
  (bind _hitactor (CallFunction|TracetoFindInventoryActor))
  ;[1 1 1] Simple Demo Actions w/o Project Inputs For Ease Of Migration
  ;;[1 1 1] Attempt to interact with a forward facing actor that has our InventoryCore Interface implemented
  (:Pressed
    (Utilities|IsValid _hitactor
      (:Is%20Valid
        (bind _interactallowed (Class|InventoryInterfaceCore|GetInteractAllowed(Message) _hitactor))
        (if _interactallowed
          (CallFunction|ServerEventInteractRequest _hitactor))))))

(event Input|KeyboardEvents|R
  (params (Key :type Key%20Structure))
  (bind _hitactor (CallFunction|TracetoFindInventoryActor))
  ;[1 1 1] Simple Demo Actions w/o Project Inputs For Ease Of Migration
  ;;[1 1 1] Attempt to interact with a forward facing actor that has our InventoryCore Interface implemented
  (:Pressed
    (Utilities|IsValid _hitactor
      (:Is%20Valid
        (bind _interactallowed (Class|InventoryInterfaceCore|GetInteractAllowed(Message) _hitactor))
        (if _interactallowed
          (CallFunction|ServerEventInteractRequest _hitactor))))))

(fn ConstructionScript)

(fn TracetoFindInventoryActor
  (bind _camera (Variables|Default|GetCamera))
  (bind _returnvalue (Transformation|GetWorldLocation _camera))
  (bind (_outhit _returnvalue_2) (Collision|LineTraceByChannel _returnvalue (+ _returnvalue (* (Math|Vector|GetForwardVector (Transformation|GetWorldRotation _camera)) 5e+02)) "TraceTypeQuery1" false (Utilities|Array|MakeArray self) "ForDuration" true "(R=1.000000,G=0.000000,B=0.000000,A=1.000000)" "(R=0.000000,G=1.000000,B=0.000000,A=1.000000)" 2.0))
  (if _returnvalue_2
    (if (Utilities|DoesObjectImplementInterface (.HitActor (Collision|BreakHitResult _outhit)) "/Game/BPInventory/InventoryCore/Interface/InventoryInterfaceCore.InventoryInterfaceCore_C")
      (return (.HitActor (Collision|BreakHitResult _outhit)))
      (else
        _)))
  (return 0))

(fn ClientFuncReceivedInventoryWidgetResponse
  (params (Owned%20Handler :type AC%20Inventory%20Handler%20Object%20Reference) (Other%20Handler :type AC%20Inventory%20Handler%20Object%20Reference))
  (bind _returnvalue (Game|GetPlayerController 0))
  (Default|ClientEventRemoveInventoryWidget Owned%20Handler)
  (bind _inventory_widget (Default|ClientFuncGetInventoryWidget Other%20Handler))
  (bind _inventory_widget_2 (Default|ClientFuncGetInventoryWidget Owned%20Handler))
  (bind _asw_inventory_main_example (Utilities|Casting|CastToW_InventoryMain_Example _inventory_widget_2))
  (Widget|Panel|ClearChildren (Variables|/Game/BPInventory/InventoryExample/UI/W_InventoryMain_Example.W_InventoryMain_Example_C|GetOtherWidgetBorder _asw_inventory_main_example))
  (Widget|Panel|AddChild (Variables|/Game/BPInventory/InventoryExample/UI/W_InventoryMain_Example.W_InventoryMain_Example_C|GetOtherWidgetBorder _asw_inventory_main_example) _inventory_widget)
  (Class|InventoryInterfaceCore|ClientFuncReceiveInventoryData(Message) _inventory_widget (Variables|/Game/BPInventory/InventoryCore/Components/AC_InventoryHandler.AC_InventoryHandler_C|GetMain%20Inventory Other%20Handler) (Variables|/Game/BPInventory/InventoryCore/Components/AC_InventoryHandler.AC_InventoryHandler_C|GetEquipped%20Inventory Other%20Handler))
  (bind _inventory_widget_3 (Default|ClientFuncGetInventoryWidget Owned%20Handler))
  (if (not (Widget|IsVisible _inventory_widget_3))
    (UserInterface|Viewport|AddtoViewport _inventory_widget_3 0)
    (Input|SetInputModeGameandUI _returnvalue 0 "DoNotLock" true false)
    (Variables|/Script/Engine.PlayerController|SetbShowMouseCursor _returnvalue true)))

(fn ClientFuncReceivedTransactionWidgetResponse
  (params (Owned%20Handler :type AC%20Inventory%20Handler%20Object%20Reference) (Transaction%20Handler :type AC%20Inventory%20Handler%20Object%20Reference))
  (bind _returnvalue (Game|GetPlayerController 0))
  (switch Utilities|FlowControl|Switch|SwitchonInventoryCompType (Variables|/Game/BPInventory/InventoryCore/Components/AC_InventoryHandler.AC_InventoryHandler_C|GetComponent%20Type Transaction%20Handler)
    (:NewEnumerator0
      (Default|ClientEventRemoveInventoryWidget Owned%20Handler :!label _label))
    (:NewEnumerator1
      (goto _label))
    (:NewEnumerator2
      _))
  (bind _inventory_widget (Default|ClientFuncGetInventoryWidget Owned%20Handler))
  (bind _transaction_widget (Default|ClientFuncGetTransactionWidget Owned%20Handler Transaction%20Handler))
  (bind _asw_inventory_main_example (Utilities|Casting|CastToW_InventoryMain_Example _inventory_widget))
  (Widget|Panel|ClearChildren (Variables|/Game/BPInventory/InventoryExample/UI/W_InventoryMain_Example.W_InventoryMain_Example_C|GetTransactionWidgetBorder _asw_inventory_main_example))
  (Widget|Panel|AddChild (Variables|/Game/BPInventory/InventoryExample/UI/W_InventoryMain_Example.W_InventoryMain_Example_C|GetTransactionWidgetBorder _asw_inventory_main_example) _transaction_widget)
  (if (not (Widget|IsVisible _inventory_widget))
    (UserInterface|Viewport|AddtoViewport _inventory_widget 0)
    (Input|SetInputModeGameandUI _returnvalue 0 "DoNotLock" true false)
    (Variables|/Script/Engine.PlayerController|SetbShowMouseCursor _returnvalue true)))

(fn ClientFuncReceiveInventoryData
  (params (Main%20Inventory :type Array%20of%20Inventory%20Item%20Replicated%20Structures) (Equipped%20Inventory :type Array%20of%20Inventory%20Item%20Replicated%20Structures))
  (return false))

(fn ClientFuncReceiveItemData
  (params (Array%20Type :type InventoryArrayType%20Enum :default "NewEnumerator0") (Index :type Integer) (Inventory%20Item%20Replicated :type Inventory%20Item%20Replicated%20Structure))
  (return false))

(fn ClientFuncReceiveTransactionData
  (params (TransactionList :type Array%20of%20Slot%20Information%20Structures))
  (return false))

(fn ClientFuncSendInitialDatatoInventoryWidget
  (params (Inventory%20Handler :type AC%20Inventory%20Handler%20Object%20Reference) (Equipped%20Type%20Array :type Array%20of%20Byte%20Array%20Structures))
  (return false))

(fn ClientFuncSendInitialDatatoTransactionWidget
  (params (Owned%20Inventory%20Handler :type AC%20Inventory%20Handler%20Object%20Reference) (Transacting%20Inventory%20Handler :type AC%20Inventory%20Handler%20Object%20Reference))
  (return false))

(fn GetInteractAllowed
  (bind _inventory_handler (Class|InventoryInterfaceCore|GetInventoryHandler(Message) (Variables|GetPlayerState)))
  (return (CallFunction|IsHandlerStateSafe _inventory_handler)))

(fn GetInventoryHandler
  (bind _inventory_handler (Class|InventoryInterfaceCore|GetInventoryHandler(Message) (Variables|GetPlayerState)))
  (return _inventory_handler))

(fn GetInventoryItemReplicatedData
  (return ""))

(fn ServerFuncInteractionStarted
  (params (Handler%20A :type AC%20Inventory%20Handler%20Object%20Reference) (Handler%20B :type AC%20Inventory%20Handler%20Object%20Reference))
  (return false))

(fn ServerFuncInteractRequest
  (params (Sender :type Actor%20Object%20Reference))
  (bind _inventory_handler (Class|InventoryInterfaceCore|GetInventoryHandler(Message) Sender))
  (Utilities|IsValid _inventory_handler
    (:Is%20Valid
      (bind _inventory_handler_2 (Class|InventoryInterfaceCore|GetInventoryHandler(Message) (Variables|GetPlayerState)))
      (Utilities|IsValid _inventory_handler_2
        (:Is%20Valid
          (bind _success (Default|ServerFuncHandlerInteraction _inventory_handler _inventory_handler_2))
          (return _success))))))

(fn ServerFuncInventoryInitialized
  (params (Inventory%20Handler :type AC%20Inventory%20Handler%20Object%20Reference))
  (return true))

(fn ServerFuncInventoryItemDeleted
  (params (Deleted%20Item%20Data :type Inventory%20Item%20Replicated%20Structure))
  (return false))

(fn ServerFuncInventoryItemObtained
  (params (Obtained%20Item%20Data :type Inventory%20Item%20Replicated%20Structure))
  (bind (_coredatareference _currentstackcount) (Utilities|Struct|BreakInventoryItemReplicated Obtained%20Item%20Data))
  (Development|PrintString (Utilities|String|Append "obtained = " (Utilities|String|ToString(Name) (.RowName (Utilities|Struct|BreakDataTableRowHandle _coredatareference))) " - " (Utilities|String|ToString(Integer) _currentstackcount)))
  (return false))

(fn ServerFuncInventoryItemProductionResult
  (params (Production%20Successful :type Boolean) (Production%20Data%20Table%20Row :type Data%20Table%20Row%20Handle%20Structure) (Produced%20Items :type Array%20of%20Inventory%20Item%20Replicated%20Structures))
  (return false))

(fn ServerFuncInventorySlotDropped
  (params (Inventory%20Item%20Replicated :type Inventory%20Item%20Replicated%20Structure))
  (bind _returnvalue (Transformation|GetActorLocation))
  (bind _returnvalue_2 (Math|Random|RandomFloatinRange -25.0 25.0))
  (bind _returnvalue_3 (Game|SpawnActorfromClass :Class "/Game/BPInventory/InventoryExample/Blueprints/BP_DroppedItem.BP_DroppedItem_C" :SpawnTransform (Math|Transform|MakeTransform (Math|Vector|MakeVector (+ (.x _returnvalue) _returnvalue_2) (+ (.y _returnvalue) _returnvalue_2) (.z _returnvalue)) (Math|Random|RandomRotator false) "1.000000,1.000000,1.000000") :CollisionHandlingOverride "AdjustIfPossibleButAlwaysSpawn" :Inventory%20Item%20Replicated Inventory%20Item%20Replicated :Instigator 0))
  (return (Utilities|IsValid _returnvalue_3)))

(fn ServerFuncInventorySlotStateChange
  (params (Inventory%20Handler :type AC%20Inventory%20Handler%20Object%20Reference) (Array%20Type :type InventoryArrayType%20Enum :default "NewEnumerator0") (Index :type Integer) (Valid%20Item :type Boolean) (Inventory%20Item%20Replicated :type Inventory%20Item%20Replicated%20Structure))
  (return true))

(fn ServerFuncInventorySlotValueChange
  (params (Inventory%20Handler :type AC%20Inventory%20Handler%20Object%20Reference) (Array%20Type :type InventoryArrayType%20Enum :default "NewEnumerator0") (Index :type Integer) (Inventory%20Item%20Replicated :type Inventory%20Item%20Replicated%20Structure))
  (return true))

(fn ServerFuncTransactionStarted
  (params (Handler%20A :type AC%20Inventory%20Handler%20Object%20Reference) (Handler%20B :type AC%20Inventory%20Handler%20Object%20Reference))
  (return false))

(fn SetInventoryItemReplicatedData
  (params (InventoryItemReplicated :type Inventory%20Item%20Replicated%20Structure))
  (return false))