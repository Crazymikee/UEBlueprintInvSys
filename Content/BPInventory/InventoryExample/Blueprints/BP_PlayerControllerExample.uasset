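; Example player controller for the inventory system that registers the inventory's input bindings at runtime.
; On BeginPlay, the Remote branch of an authority switch, fed by standalone and authority checks, calls the client setup function.
; That function walks the InputMap, adds an action mapping to Input Settings for each name not already mapped, then saves the key mappings.
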(event EventBeginPlay
  (Utilities|AuthoritySwitch (Class|KismetSystemLibrary|IsStandalone) (Ability|HasAuthority)
    (:Remote
      (CallFunction|ClientFuncSetupInventoryInputs))))

(fn ConstructionScript)

(fn ClientFuncSetupInventoryInputs
  (bind _returnvalue (Class|InputSettings|GetInputSettings))
  (bind _inputmap (LocalVariables|GetInputMap))
  (bind _keys (Utilities|Map|Keys _inputmap))
  (bind _values (Utilities|Map|Values _inputmap))
  (for (_array_element _array_index) _keys
    (if (not (Utilities|Array|IsValidIndex (Class|InputSettings|GetActionMappingbyName _returnvalue _array_element)))
      (Class|InputSettings|AddActionMapping _returnvalue (Utilities|Struct|MakeInputActionKeyMapping _array_element (.bshift (Utilities|Array|Get(acopy) _values _array_index)) (.bctrl (Utilities|Array|Get(acopy) _values _array_index)) (.balt (Utilities|Array|Get(acopy) _values _array_index)) (.bcmd (Utilities|Array|Get(acopy) _values _array_index)) (.key (Utilities|Array|Get(acopy) _values _array_index))) true)))
  (Class|InputSettings|SaveKeyMappings _returnvalue))