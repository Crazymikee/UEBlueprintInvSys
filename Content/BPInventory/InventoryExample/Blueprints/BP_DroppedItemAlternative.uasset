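; Dropped inventory item actor that players pick up, with its logic held in a DroppedItemHandler component seeded in the construction script.
; The handler's item response adds a physics-simulated static or skeletal mesh from item data, optionally looping an animation, and attaches the widget to it.
; Interact requests add the item to the sender's inventory, using a PickupAttempted lock and destroying the actor unless some count remains.
; Invalid items also destroy it.
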(event InventoryItemInvalid(DroppedItemHandler)
  (Actor|DestroyActor))

(event InventoryItemRepResponse(DroppedItemHandler)
  (params (InventoryItemReplicated :type Inventory%20Item%20Replicated%20Structure))
  (Core|InventoryItemRepResponse InventoryItemReplicated))

(fn ConstructionScript
  (bind _droppeditemhandler (Variables|Default|GetDroppedItemHandler))
  (Variables|/Game/BPInventory/InventoryCore/Components/DroppedItemHandler.DroppedItemHandler_C|SetDefault%20Item%20Data _droppeditemhandler (Variables|Settings|GetDefault%20Item%20Data))
  (Variables|/Game/BPInventory/InventoryCore/Components/DroppedItemHandler.DroppedItemHandler_C|SetDefault%20Stack%20Count _droppeditemhandler (Variables|Settings|GetDefault%20Stack%20Count))
  (Variables|/Game/BPInventory/InventoryCore/Components/DroppedItemHandler.DroppedItemHandler_C|SetDefault%20Rarity%20Override _droppeditemhandler (Variables|Settings|GetDefault%20Rarity%20Override))
  (Variables|/Game/BPInventory/InventoryCore/Components/DroppedItemHandler.DroppedItemHandler_C|SetInventory%20Item%20Replicated _droppeditemhandler (Variables|Core|GetInventory%20Item%20Replicated)))

(fn InventoryItemRepResponse
  (params (InventoryItemReplicated :type Inventory%20Item%20Replicated%20Structure))
  (bind (_found _inventory_item_core) (CallFunction|GetItemCoreData InventoryItemReplicated))
  (bind _customdata (Utilities|Struct|BreakInventoryItemCore _inventory_item_core))
  (bind (_gamespecificdata _droppedstaticmesh _droppedskeletalmesh _droppedskeletalmontage) (Utilities|Struct|BreakCustomItemDataCore _customdata))
  (if _found
    (Utilities|IsValid _droppedstaticmesh
      (:Is%20Valid
        (bind _returnvalue (AddComponent|AddStaticMeshComponent false))
        (Transformation|AttachComponentToComponent _returnvalue (Variables|Default|GetDefaultSceneRoot) "None" "SnapToTarget" "SnapToTarget" "SnapToTarget" true)
        (Class|PrimitiveComponent|SetAllUseCCD _returnvalue true)
        (Collision|SetCollisionResponsetoChannel _returnvalue "ECC_Pawn" "ECR_Overlap")
        (Transformation|AttachComponentToComponent (Variables|Default|GetWidget) _returnvalue "None" "SnapToTarget" "SnapToTarget" "SnapToTarget" true)
        (Components|StaticMesh|SetStaticMesh _returnvalue _droppedstaticmesh)
        (Physics|SetSimulatePhysics _returnvalue true))
      (:Is%20Not%20Valid
        _))
    (Utilities|IsValid _droppedskeletalmesh
      (:Is%20Valid
        (bind _returnvalue_2 (AddComponent|AddSkeletalMeshComponent false))
        (Transformation|AttachComponentToComponent _returnvalue_2 (Variables|Default|GetDefaultSceneRoot) "None" "SnapToTarget" "SnapToTarget" "SnapToTarget" true)
        (Class|PrimitiveComponent|SetAllUseCCD _returnvalue_2 true)
        (Collision|SetCollisionResponsetoChannel _returnvalue_2 "ECC_Pawn" "ECR_Overlap")
        (Transformation|AttachComponentToComponent (Variables|Default|GetWidget) _returnvalue_2 "None" "SnapToTarget" "SnapToTarget" "SnapToTarget" true)
        (Components|SkinnedMesh|SetSkinnedAssetandUpdate _returnvalue_2 _droppedskeletalmesh true)
        (Physics|SetSimulatePhysics _returnvalue_2 true)
        (Utilities|IsValid _droppedskeletalmontage
          (:Is%20Valid
            (Components|Animation|SetAnimationMode _returnvalue_2 "AnimationSingleNode" true)
            (Components|Animation|PlayAnimation _returnvalue_2 _droppedskeletalmontage true)))))))

(fn ClientFuncGetSlotInfoWidget
  (params (Slot%20Info :type Slot%20Information%20Structure))
  (return 0))

(fn ClientFuncReceivedHandlerResponse
  (params (Owned%20Handler :type Inventory%20Handler%20Object%20Reference) (Other%20Handler :type Inventory%20Handler%20Object%20Reference))
  (return false))

(fn ClientFuncReceiveInventoryData
  (params (Main%20Inventory :type Array%20of%20Inventory%20Item%20Replicated%20Structures) (Equipped%20Inventory :type Array%20of%20Inventory%20Item%20Replicated%20Structures))
  (return false))

(fn ClientFuncReceiveItemData
  (params (Array%20Type :type InventoryArrayType%20Enum :default "NewEnumerator0") (Index :type Integer) (Inventory%20Item%20Replicated :type Inventory%20Item%20Replicated%20Structure))
  (Class|InventoryInterfaceCore|ClientFuncReceiveItemData(Message) (UserInterface|GetUserWidgetObject (Variables|Default|GetWidget)) Array%20Type Index Inventory%20Item%20Replicated)
  (return false))

(fn ClientFuncSendInitialDatatoInventoryWidget
  (params (Inventory%20Handler :type Inventory%20Handler%20Object%20Reference) (Equipped%20Type%20Array :type Array%20of%20Byte%20Array%20Structures))
  (return false))

(fn GetInteractAllowed
  (return (not (Variables|/Game/BPInventory/InventoryCore/Components/DroppedItemHandler.DroppedItemHandler_C|GetPickupAttempted (Variables|Default|GetDroppedItemHandler)))))

(fn GetInventoryHandler
  (return 0))

(fn GetInventoryItemReplicatedData
  (return (Variables|/Game/BPInventory/InventoryCore/Components/DroppedItemHandler.DroppedItemHandler_C|GetInventory%20Item%20Replicated (Variables|Default|GetDroppedItemHandler))))

(fn ServerFuncInteractRequest
  (params (Sender :type Actor%20Object%20Reference))
  (bind _droppeditemhandler (Variables|Default|GetDroppedItemHandler))
  (bind _inventory_handler (Class|InventoryInterfaceCore|GetInventoryHandler(Message) Sender))
  (bind _interactallowed (CallFunction|GetInteractAllowed))
  (if _interactallowed
    (Variables|/Game/BPInventory/InventoryCore/Components/DroppedItemHandler.DroppedItemHandler_C|SetPickupAttempted _droppeditemhandler true)
    (bind (_success _dropped_actor_has_count) (Default|ServerFuncAddItemBlind _inventory_handler (Variables|/Game/BPInventory/InventoryCore/Components/DroppedItemHandler.DroppedItemHandler_C|GetInventory%20Item%20Replicated _droppeditemhandler) self false "NewEnumerator0"))
    (if _success
      (if _dropped_actor_has_count
        (Variables|/Game/BPInventory/InventoryCore/Components/DroppedItemHandler.DroppedItemHandler_C|SetPickupAttempted (Variables|Default|GetDroppedItemHandler) false)
        (else
          (Actor|DestroyActor)))
      (return true)
      (else
        (Variables|/Game/BPInventory/InventoryCore/Components/DroppedItemHandler.DroppedItemHandler_C|SetPickupAttempted (Variables|Default|GetDroppedItemHandler) false)
        (return false)))))

(fn ServerFuncInventoryInitialized
  (params (Inventory%20Handler :type Inventory%20Handler%20Object%20Reference))
  (return false))

(fn ServerFuncInventoryItemDeleted
  (params (Deleted%20Item%20Data :type Inventory%20Item%20Replicated%20Structure))
  (return false))

(fn ServerFuncInventoryItemObtained
  (params (Obtained%20Item%20Data :type Inventory%20Item%20Replicated%20Structure))
  (return false))

(fn ServerFuncInventoryItemProductionResult
  (params (Production%20Successful :type Boolean) (Production%20Data%20Table%20Row :type Data%20Table%20Row%20Handle%20Structure) (Produced%20Items :type Array%20of%20Inventory%20Item%20Replicated%20Structures))
  (return false))

(fn ServerFuncInventorySlotDropped
  (params (Inventory%20Item%20Replicated :type Inventory%20Item%20Replicated%20Structure))
  (return false))

(fn ServerFuncInventorySlotStateChange
  (params (Inventory%20Handler :type Inventory%20Handler%20Object%20Reference) (Array%20Type :type InventoryArrayType%20Enum :default "NewEnumerator0") (Index :type Integer) (Valid%20Item :type Boolean) (Inventory%20Item%20Replicated :type Inventory%20Item%20Replicated%20Structure))
  (return false))

(fn ServerFuncInventorySlotValueChange
  (params (Inventory%20Handler :type Inventory%20Handler%20Object%20Reference) (Array%20Type :type InventoryArrayType%20Enum :default "NewEnumerator0") (Index :type Integer) (Inventory%20Item%20Replicated :type Inventory%20Item%20Replicated%20Structure))
  (return false))

(fn SetInventoryItemReplicatedData
  (params (InventoryItemReplicated :type Inventory%20Item%20Replicated%20Structure))
  (Variables|/Game/BPInventory/InventoryCore/Components/DroppedItemHandler.DroppedItemHandler_C|SetInventory%20Item%20Replicated (Variables|Default|GetDroppedItemHandler) InventoryItemReplicated)
  (return true))