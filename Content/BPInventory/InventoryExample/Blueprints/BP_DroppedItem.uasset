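; Replicated world pickup actor for a dropped inventory item.
; The server generates item data from defaults or uses assigned data, destroying itself if neither is valid.
; Item data spawns a physics-simulated static or skeletal mesh, with optional looping animation, and feeds the attached widget; clients poll until data arrives.
; Interaction adds the item to the sender's InventoryHandler behind a PickupAttempted guard, destroying the actor unless count remains.
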(event EventBeginPlay
  (bind _default_item_data (Variables|Settings|GetDefault%20Item%20Data))
  (bind _default_stack_count (Variables|Settings|GetDefault%20Stack%20Count))
  (bind _default_rarity_override (Variables|Settings|GetDefault%20Rarity%20Override))
  (bind (_valid _inventory_item_replicated) (CallFunction|GenerateItemData _default_item_data _default_stack_count _default_rarity_override))
  (Utilities|AuthoritySwitch (Class|KismetSystemLibrary|IsStandalone) (Ability|HasAuthority)
    (:Authority
      (if _valid
        (Variables|Core|SetInventory%20Item%20Replicated _inventory_item_replicated)
        (elif (CallFunction|CheckValidItem (Variables|Core|GetInventory%20Item%20Replicated))
          (Core|Item|InventoryItemRepResponse (Variables|Core|GetInventory%20Item%20Replicated))
          (else
            (Actor|DestroyActor)))))
    (:Remote
      (if (CallFunction|CheckValidItem (Variables|Core|GetInventory%20Item%20Replicated)) :!label _label
        (Class|InventoryInterfaceCore|ClientFuncReceiveItemData(Message) (UserInterface|GetUserWidgetObject (Variables|Default|GetWidget)) "NewEnumerator0" -1 (Variables|Core|GetInventory%20Item%20Replicated))
        (else
          (Utilities|FlowControl|Delay 0.0)
          (goto _label))))))

(fn ConstructionScript)

(fn OnRepInventoryItemReplicated
  (bind _inventory_item_replicated (Variables|Core|GetInventory%20Item%20Replicated))
  (Core|Item|InventoryItemRepResponse _inventory_item_replicated)
  (Class|InventoryInterfaceCore|ClientFuncReceiveItemData(Message) (UserInterface|GetUserWidgetObject (Variables|Default|GetWidget)) "NewEnumerator0" -1 _inventory_item_replicated))

(fn InventoryItemRepResponse
  (params (InventoryItemReplicated :type Inventory%20Item%20Replicated%20Structure))
  (bind (_found _inventory_item_core) (CallFunction|GetItemCoreData InventoryItemReplicated))
  (bind _customdata (Utilities|Struct|BreakInventoryItemCore _inventory_item_core))
  (bind (_gamespecificdata _droppedstaticmesh _droppedskeletalmesh _droppedskeletalmontage) (Utilities|Struct|BreakCustomItemDataCore _customdata))
  (if _found
    (Utilities|IsValid _droppedstaticmesh
      (:Is%20Valid
        (bind _returnvalue (AddComponent|AddStaticMeshComponent false))
        (Transformation|AttachComponentToComponent _returnvalue (Variables|Default|GetDefaultSceneRoot) "None" "SnapToTarget" "SnapToTarget" "SnapToTarget" true)
        (Class|PrimitiveComponent|SetAllUseCCD _returnvalue true)
        (Collision|SetCollisionResponsetoChannel _returnvalue "ECC_Pawn" "ECR_Overlap")
        (Transformation|AttachComponentToComponent (Variables|Default|GetWidget) _returnvalue "None" "SnapToTarget" "SnapToTarget" "SnapToTarget" true)
        (Components|StaticMesh|SetStaticMesh _returnvalue _droppedstaticmesh)
        (Physics|SetSimulatePhysics _returnvalue true))
      (:Is%20Not%20Valid
        _))
    (Utilities|IsValid _droppedskeletalmesh
      (:Is%20Valid
        (bind _returnvalue_2 (AddComponent|AddSkeletalMeshComponent false))
        (Transformation|AttachComponentToComponent _returnvalue_2 (Variables|Default|GetDefaultSceneRoot) "None" "SnapToTarget" "SnapToTarget" "SnapToTarget" true)
        (Class|PrimitiveComponent|SetAllUseCCD _returnvalue_2 true)
        (Collision|SetCollisionResponsetoChannel _returnvalue_2 "ECC_Pawn" "ECR_Overlap")
        (Transformation|AttachComponentToComponent (Variables|Default|GetWidget) _returnvalue_2 "None" "SnapToTarget" "SnapToTarget" "SnapToTarget" true)
        (Components|SkinnedMesh|SetSkinnedAssetandUpdate _returnvalue_2 _droppedskeletalmesh true)
        (Physics|SetSimulatePhysics _returnvalue_2 true)
        (Utilities|IsValid _droppedskeletalmontage
          (:Is%20Valid
            (Components|Animation|SetAnimationMode _returnvalue_2 "AnimationSingleNode" true)
            (Components|Animation|PlayAnimation _returnvalue_2 _droppedskeletalmontage true)))))))

(fn ClientFuncGetSlotInfoWidget
  (params (Slot%20Info :type Slot%20Information%20Structure))
  (return 0))

(fn ClientFuncReceivedHandlerResponse
  (params (Owned%20Handler :type Inventory%20Handler%20Object%20Reference) (Other%20Handler :type Inventory%20Handler%20Object%20Reference))
  (return false))

(fn ClientFuncReceiveInventoryData
  (params (Main%20Inventory :type Array%20of%20Inventory%20Item%20Replicated%20Structures) (Equipped%20Inventory :type Array%20of%20Inventory%20Item%20Replicated%20Structures))
  (return false))

(fn ClientFuncReceiveItemData
  (params (Array%20Type :type InventoryArrayType%20Enum :default "NewEnumerator0") (Index :type Integer) (Inventory%20Item%20Replicated :type Inventory%20Item%20Replicated%20Structure))
  (return false))

(fn ClientFuncSendInitialDatatoInventoryWidget
  (params (Inventory%20Handler :type Inventory%20Handler%20Object%20Reference) (Equipped%20Type%20Array :type Array%20of%20Byte%20Array%20Structures))
  (return false))

(fn GetInteractAllowed
  (return (not (Variables|Core|GetPickupAttempted))))

(fn GetInventoryHandler
  (return 0))

(fn GetInventoryItemReplicatedData
  (return (Variables|Core|GetInventory%20Item%20Replicated)))

(fn ServerFuncInteractRequest
  (params (Sender :type Actor%20Object%20Reference))
  (bind _interactallowed (CallFunction|GetInteractAllowed))
  (if _interactallowed
    (Variables|Core|SetPickupAttempted true)
    (bind (_success _dropped_actor_has_count) (Default|ServerFuncAddItemBlind (Actor|GetComponentbyClass Sender "/Game/BPInventory/InventoryCore/Components/InventoryHandler.InventoryHandler_C") (Variables|Core|GetInventory%20Item%20Replicated) self false "NewEnumerator0"))
    (if _success
      (if _dropped_actor_has_count
        (Variables|Core|SetPickupAttempted false)
        (else
          (Actor|DestroyActor)))
      (return true)
      (else
        (Variables|Core|SetPickupAttempted false)
        (return false)))))

(fn ServerFuncInventoryInitialized
  (params (Inventory%20Handler :type Inventory%20Handler%20Object%20Reference))
  (return false))

(fn ServerFuncInventoryItemDeleted
  (params (Deleted%20Item%20Data :type Inventory%20Item%20Replicated%20Structure))
  (return false))

(fn ServerFuncInventoryItemObtained
  (params (Obtained%20Item%20Data :type Inventory%20Item%20Replicated%20Structure))
  (return false))

(fn ServerFuncInventoryItemProductionResult
  (params (Production%20Successful :type Boolean) (Production%20Data%20Table%20Row :type Data%20Table%20Row%20Handle%20Structure) (Produced%20Items :type Array%20of%20Inventory%20Item%20Replicated%20Structures))
  (return false))

(fn ServerFuncInventorySlotDropped
  (params (Inventory%20Item%20Replicated :type Inventory%20Item%20Replicated%20Structure))
  (return false))

(fn ServerFuncInventorySlotStateChange
  (params (Inventory%20Handler :type Inventory%20Handler%20Object%20Reference) (Array%20Type :type InventoryArrayType%20Enum :default "NewEnumerator0") (Index :type Integer) (Valid%20Item :type Boolean) (Inventory%20Item%20Replicated :type Inventory%20Item%20Replicated%20Structure))
  (return false))

(fn ServerFuncInventorySlotValueChange
  (params (Inventory%20Handler :type Inventory%20Handler%20Object%20Reference) (Array%20Type :type InventoryArrayType%20Enum :default "NewEnumerator0") (Index :type Integer) (Inventory%20Item%20Replicated :type Inventory%20Item%20Replicated%20Structure))
  (return false))

(fn SetInventoryItemReplicatedData
  (params (InventoryItemReplicated :type Inventory%20Item%20Replicated%20Structure))
  (Variables|Core|SetInventory%20Item%20Replicated InventoryItemReplicated)
  (return true))