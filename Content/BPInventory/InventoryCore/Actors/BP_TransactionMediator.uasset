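; Replicated actor that mediates an item transaction between two inventory handlers, A and B, each with its own transaction list.
; Validation walks both lists in reverse, removing items their handler no longer holds and forcing a net update, and fails only if a handler is invalid.
; Item checks use dictionary indices for main and equipped inventories, then compare whole structs.
; The BeginPlay controller check and both RepNotifies are empty stubs.
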(event EventBeginPlay
  (|CallParentFunction)
  (if (and (.Valid (CallFunction|GetControllerfromInventoryHandler (Variables|Default|GetA%20Handler))) (.Valid (CallFunction|GetControllerfromInventoryHandler (Variables|Default|GetB%20Handler))))
    _))

(fn ConstructionScript)

(fn DoesIdenticalItemExist
  (params (Handler :type Inventory%20Handler%20Object%20Reference) (Inventory%20Item%20Replicated :type Inventory%20Item%20Replicated%20Structure))
  (bind _coredatareference (Utilities|Struct|BreakInventoryItemReplicated Inventory%20Item%20Replicated))
  (Utilities|FlowControl|Sequence
    (:then_0
      (for _index (range 0 1)
        (if (.ReturnValue (Utilities|Map|Find (Utilities|Select :Index _index :Option%200 (Variables|/Game/BPInventory/InventoryCore/Components/InventoryHandler.InventoryHandler_C|GetDictionary%20Item%20Index%20Inv Handler) :Option%201 (Variables|/Game/BPInventory/InventoryCore/Components/InventoryHandler.InventoryHandler_C|GetDictionary%20Item%20Index%20Equip Handler)) (Utilities|Struct|MakeDictionaryDataTableInfo (.rowname _coredatareference) (.datatable _coredatareference))))
          (for _array_element (.integers (.Value (Utilities|Map|Find (Utilities|Select :Index _index :Option%200 (Variables|/Game/BPInventory/InventoryCore/Components/InventoryHandler.InventoryHandler_C|GetDictionary%20Item%20Index%20Inv Handler) :Option%201 (Variables|/Game/BPInventory/InventoryCore/Components/InventoryHandler.InventoryHandler_C|GetDictionary%20Item%20Index%20Equip Handler)) (Utilities|Struct|MakeDictionaryDataTableInfo (.rowname _coredatareference) (.datatable _coredatareference)))))
            (if (Utilities|Array|Identical (Utilities|Array|MakeArray (Utilities|Array|Get(acopy) (Utilities|Select :Index _index :Option%200 (Variables|/Game/BPInventory/InventoryCore/Components/InventoryHandler.InventoryHandler_C|GetMain%20Inventory Handler) :Option%201 (Variables|/Game/BPInventory/InventoryCore/Components/InventoryHandler.InventoryHandler_C|GetEquipped%20Inventory Handler)) _array_element)) (Utilities|Array|MakeArray Inventory%20Item%20Replicated))
              (return true))))))
    (:then_1
      (return false))))

(fn ValidateTransactionList
  (if (and (Utilities|IsValid (Variables|Default|GetA%20Handler)) (Utilities|IsValid (Variables|Default|GetB%20Handler)))
    (for _index (range 0 1)
      (bind (_arrayindex _arrayelement) (Utilities|Array|ReverseforEachLoop (Utilities|Select :Index _index :Option%200 (Variables|Default|GetATransactionList) :Option%201 (Variables|Default|GetBTransactionList)))
        (:LoopBody
          (bind _return_value (CallFunction|DoesIdenticalItemExist (Utilities|Select :Index _index :Option%200 (Variables|Default|GetA%20Handler) :Option%201 (Variables|Default|GetB%20Handler)) _arrayelement))
          (if (not _return_value)
            (Utilities|Array|RemoveIndex (Utilities|Select :Index _index :Option%200 (Variables|Default|GetATransactionList) :Option%201 (Variables|Default|GetBTransactionList)) _arrayindex)
            (Networking|ForceNetUpdate)))))
    (return true)
    (else
      (return false))))

(fn OnRepATransactionList)

(fn OnRepBTransactionList)